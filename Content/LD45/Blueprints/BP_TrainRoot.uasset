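; Train root actor that simulates a metro ride along a station list, reversing at either end.
; A timeline advances PositionInLine between stops and triggers next-station and exit-side announcements.
; At stops it shows the station name and cycles the left doors through the GameMode, then departs.
; While riding, layered Perlin noise bobs the actor vertically, and speed and position feed a window material parameter collection to fake travel.
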(event `self.ReceiveBeginPlay`
  (set `self.OriginalPos` (`self.K2_GetActorLocation`))
  (`self.BeginNextStationEvent`))

(event `self.ReceiveTick`
  (params (DeltaSeconds :type "Float (single-precision)"))
  (`self.WobbleTrainFX`))

(event `BeginStationEvent`
  (bind _asbp_third_person_game_mode (cast `/Game/ThirdPerson/Blueprints/BP_ThirdPersonGameMode` (`GameplayStatics.GetGameMode`) :!pure true))
  (set `self.Riding` false)
  (`|ExecutionSequence`
    (:`then_0`
      (`TextRenderComponent.K2_SetText` (`self.TextRender`) (`.Name_2_59C06E5E45D6AD391E46ABAF059DCFBD` (break `/Game/LD45/Blueprints/FTrainStation` (`|GetArrayItem` (`self. Stations`) (`KismetMathLibrary.FFloor` (`self.PositionInLine`))))))
      (`SceneComponent.SetVisibility` (`self.TextRender`) true false)
      (`KismetSystemLibrary.Delay` 4.0)
      (`SceneComponent.SetVisibility` (`self.TextRender`) false false))
    (:`then_1`
      (`KismetSystemLibrary.Delay` 1.0)
      (`/Game/ThirdPerson/Blueprints/BP_ThirdPersonGameMode.OpenDoor` _asbp_third_person_game_mode "NewEnumerator0")
      (`KismetSystemLibrary.Delay` 8.0)
      (`/Game/ThirdPerson/Blueprints/BP_ThirdPersonGameMode.CloseDoor` _asbp_third_person_game_mode "NewEnumerator0")
      ;[0.1354 0.0146 0] GoBack Logic
      (`|ExecutionSequence`
        (:`then_0`
          (if (and (== (`KismetMathLibrary.FFloor` (`self.PositionInLine`)) (`KismetArrayLibrary.Array_LastIndex` (`self. Stations`))) (not (`self.GoingBack`)))
            (set `self.GoingBack` true)))
        (:`then_1`
          (if (and (== (`self.PositionInLine`) 0.0) (`self.GoingBack`))
            (set `self.GoingBack` false)))
        (:`then_2`
          (`KismetSystemLibrary.Delay` 0.2)
          (`self.BeginNextStationEvent`))))))

(event `BeginNextStationEvent`
  (bind _positioninline (`self.PositionInLine`))
  (bind _returnvalue (`KismetMathLibrary.FFloor` (`self.PositionInLine`)))
  (set `self.Riding` true)
  (bind (_direction _waypercentage _cosmeticspeed) (`Timeline|NextStationTimeline` :!via `PlayFromStart`)
    (:`Update`
      (set `self.PositionInLine` (+ (`KismetMathLibrary.SelectInt` (`KismetMathLibrary.FCeil` _positioninline) (`KismetMathLibrary.FFloor` _positioninline) (`self.GoingBack`)) (`KismetMathLibrary.SelectFloat` (- 0.0 _waypercentage) _waypercentage (`self.GoingBack`))))
      (set `self.CosmeticSpeed` _cosmeticspeed))
    (:`Finished`
      (`self.BeginStationEvent`))
    (:`NextStation`
      (`GameplayStatics.PlaySound2D` "/Game/LD45/Audio/SFX/SW_AnnouncerHexagonalTemple.SW_AnnouncerHexagonalTemple" 1.0 1.0 0.0 null null))
    (:`Side`
      (`GameplayStatics.PlaySound2D` (select `/Game/LD45/Blueprints/EOffboardingSide` (`.OffboardingSide_12_07F6D1604018AF0E6958799D1259D026` (break `/Game/LD45/Blueprints/FTrainStation` (`|GetArrayItem` (`self. Stations`) (`KismetMathLibrary.SelectInt` _returnvalue (+ _returnvalue 1) (`self.GoingBack`))))) :`NewEnumerator0` "/Game/LD45/Audio/SFX/SW_ExitLeft.SW_ExitLeft" :`NewEnumerator1` "/Game/LD45/Audio/SFX/SW_ExitRight.SW_ExitRight" :!type "SoundBase Object Reference") 1.0 1.0 0.0 null null))))

(fn `UserConstructionScript`)

(fn `WobbleTrainFX`
  (bind _originalpos (`self.OriginalPos`))
  (if (`self.Riding`)
    (`self.K2_SetActorLocation` (select `bool` (`self.Riding`) :`false` _originalpos :`true` (+ _originalpos (`KismetMathLibrary.MakeVector` 0.0 0.0 (* (`KismetMathLibrary.PerlinNoise1D` (* (`GameplayStatics.GetTimeSeconds`) 10.0)) 5.0 (`self.CosmeticSpeed`))) (`KismetMathLibrary.MakeVector` 0.0 0.0 (* (`KismetMathLibrary.PerlinNoise1D` (* (+ (`GameplayStatics.GetTimeSeconds`) 500.0) 0.1)) 40.0 (`self.CosmeticSpeed`))))))
    (`KismetMaterialLibrary.SetScalarParameterValue` (`self.WindowMaterialInstance`) "CosmeticSpeed" (`self.CosmeticSpeed`))
    (`KismetMaterialLibrary.SetScalarParameterValue` (`self.WindowMaterialInstance`) "Location" (* (`self.PositionInLine`) -100.0))))