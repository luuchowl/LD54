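; BP_SubwayDoor is a two-panel sliding subway door that opens and closes for its assigned side of the train.
; On BeginPlay it binds to the third-person game mode's open and close door events, acting only when the side matches DoorSide and the state needs changing.
; Both actions play a 2D sound and share one IsOpen toggle, which plays or reverses a timeline sliding the panels in opposite directions along local Y.
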(event `self.ReceiveBeginPlay`
  (bind _asbp_third_person_game_mode (cast `/Game/ThirdPerson/Blueprints/BP_ThirdPersonGameMode` (`GameplayStatics.GetGameMode`)))
  (add `/Game/ThirdPerson/Blueprints/BP_ThirdPersonGameMode.OpenDoor` _asbp_third_person_game_mode (`|CreateDelegate` :!event `OpenDoor`))
  (add `/Game/ThirdPerson/Blueprints/BP_ThirdPersonGameMode.CloseDoor` _asbp_third_person_game_mode (`|CreateDelegate` :!event `CloseDoor`)))

(event `OpenDoor`
  (params (Side :type "/Game/LD45/Blueprints/EOffboardingSide Enum" :default "NewEnumerator0"))
  (bind _isopen (`self.IsOpen`))
  (if (and (== (`KismetMathLibrary.Conv_ByteToInt` Side) (`self.DoorSide`)) (not (`self.IsOpen`)))
    (`GameplayStatics.PlaySound2D` "/Game/LD45/Audio/SFX/door_opening.door_opening" 1.0 1.0 0.0 null null)
    (set `self.IsOpen` (not _isopen) :!label _label)
    (if _isopen
      (bind (_direction _doorrelativeposition) (`Timeline|TimelineOpenDoor` :!label _label_2)
        (:`Update`
          (bind _returnvalue (`KismetMathLibrary.MakeVector` 0.0 (* _doorrelativeposition (`self.DoorMovDistance`))))
          (`SceneComponent.K2_SetRelativeLocation` (`self.Door_R`) _returnvalue false false)
          (`SceneComponent.K2_SetRelativeLocation` (`self.Door_L`) (* _returnvalue -1.0) false false)))
      (else
        (goto _label_2 :!via `Reverse`)))))

(event `CloseDoor`
  (params (Side :type "/Game/LD45/Blueprints/EOffboardingSide Enum" :default "NewEnumerator0"))
  (if (and (== (`KismetMathLibrary.Conv_ByteToInt` Side) (`self.DoorSide`)) (`self.IsOpen`))
    (`GameplayStatics.PlaySound2D` "/Game/LD45/Audio/SFX/door_closing.door_closing" 1.0 1.0 0.0 null null)
    (goto _label)))

(event `ToggleOpenDoor`
  (params (Side :type "/Game/LD45/Blueprints/EOffboardingSide Enum" :default "NewEnumerator0"))
  (if (and (`self.IsOpen`) (== Side (`KismetMathLibrary.Conv_ByteToInt` (`self.DoorSide`))))
    (`self.CloseDoor` "NewEnumerator0")
    (else
      (`self.OpenDoor` "NewEnumerator0"))))

(fn `UserConstructionScript`)