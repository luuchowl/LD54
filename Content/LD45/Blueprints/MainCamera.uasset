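; MainCamera is a camera Blueprint that becomes the player's view target after a zero-length delay on BeginPlay.
; Every tick it copies the camera component's world rotation into the player controller's control rotation.
; A Glitch event replays a timeline from the start, feeding its curve into an intensity value in the camera's post-process settings for a glitch effect.
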(event `self.ReceiveBeginPlay`
  (`KismetSystemLibrary.Delay` 0.0)
  (`PlayerController.SetViewTargetWithBlend` (`GameplayStatics.GetPlayerController` 0) self 0.0 "VTBlend_Linear" 0.0 false))

(event `self.ReceiveTick`
  (params (DeltaSeconds :type "Float (single-precision)"))
  (`Controller.SetControlRotation` (`GameplayStatics.GetPlayerController` 0) (`SceneComponent.K2_GetComponentRotation` (`self.CameraComponent`))))

(event `Glitch`
  (bind (_direction _glitch) (`Timeline|GlitchTimeline` :!via `PlayFromStart`)
    (:`Update`
      (setmembers `PostProcessSettings` :`StructRef` (`CameraComponent.PostProcessSettings` (`self.CameraComponent`)) :`SceneFringeIntensity` _glitch))))

(fn `UserConstructionScript`)